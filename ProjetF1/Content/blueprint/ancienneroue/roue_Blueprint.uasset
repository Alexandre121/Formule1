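; Blueprint for an old wheel ("roue"), holding an unfinished or disabled mobility switch; BeginPlay and Tick are empty and none of the logic runs.
; The disconnected graph would set mobility to Static, wait briefly, then switch it to Movable once when five summed Box overlap counts equal zero.
; A second orphaned chain prints that zero-overlap test for debugging before feeding the same check.
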(event EventBeginPlay
  ;[1 1 1] mobilité roue
)

(event EventTick
  (params (DeltaSeconds :type Float%20%28single-precision%29))
  ;[1 1 1] mobilité roue
)

(fn ConstructionScript)